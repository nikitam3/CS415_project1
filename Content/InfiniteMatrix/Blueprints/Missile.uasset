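; Missile is a projectile actor for InfiniteMatrix that travels along world +X, staying faster than the player.
; Each tick it reads the BP_Player pawn's ForwardSpeed, adds a fixed margin and applies a frame-time-scaled world offset.
; Overlaps on the Projectile component destroy the missile, except with BP_Player actors or any BoxComponent.
; A PlaySound2D node is left unconnected and never runs.
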(event OnComponentBeginOverlap(Projectile)
  (params (OverlappedComponent :type Primitive%20Component%20Object%20Reference) (OtherActor :type Actor%20Object%20Reference) (OtherComp :type Primitive%20Component%20Object%20Reference) (OtherBodyIndex :type Integer) (bFromSweep :type Boolean) (SweepResult :type Hit%20Result%20Structure%20%28by%20ref%29))
  (if (not (or (Utilities|ClassIsChildOf (Utilities|GetClass OtherActor) "/Game/InfiniteMatrix/Blueprints/BP_Player.BP_Player_C") (Utilities|ClassIsChildOf (Utilities|GetClass OtherComp) "/Script/Engine.BoxComponent")))
    (Actor|DestroyActor)))

(event EventBeginPlay)

(event Collision|EventActorBeginOverlap
  (params (OtherActor :type Actor%20Object%20Reference)))

(event EventTick
  (params (DeltaSeconds :type Float%20%28single-precision%29))
  (bind _asbp_player (Utilities|Casting|CastToBP_Player (Game|Player|GetPlayerPawn 0)))
  (Transformation|AddActorWorldOffset (Math|Vector|MakeVector (* DeltaSeconds (+ (Variables|/Game/InfiniteMatrix/Blueprints/BP_Player.BP_Player_C|GetForwardSpeed _asbp_player) 5e+02)) 0.0 0.0)))

(fn ConstructionScript)